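; BP_Projetil is a projectile Actor Blueprint in a test content folder, with a static mesh that is launched by a physics impulse.
; LaunchProjectile pushes the mesh along the actor's forward vector, applying the impulse as a velocity change so that mass is ignored.
; GetName and GetLocation are debug helpers that print the display name and location.
; The event graph and construction script are empty, so nothing in this Blueprint calls these functions.
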(fn `getLocation`
  (`KismetSystemLibrary.PrintString` (`KismetStringLibrary.Conv_VectorToString` (`self.K2_GetActorLocation` self))))

(fn `getName`
  (`KismetSystemLibrary.PrintString` (`KismetSystemLibrary.GetDisplayName` self)))

(fn `launchProjectile`
  (`PrimitiveComponent.AddImpulse` (`self.StaticMeshComponent`) (* (`self.GetActorForwardVector` self) 1000.0) "None" true))

(fn `UserConstructionScript`)